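; Ghost enemy character that ends the run when its capsule touches the player's capsule, flagging the death in the game instance before opening GameOver.
; Walk speed switches between patrol and follow according to the AI controller's state.
; Helper functions, not called within this file, slow it after damage and destroy it below zero health.
; Tick refreshes its health bar widget from current over maximum health.
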(event `self.ReceiveBeginPlay`
  (`self.SetPatrolSpeed`))

(event `self.ReceiveTick`
  (params (DeltaSeconds :type "Float (single-precision)"))
  (`self.UpdateHealthbar`))

(event `self.OnEnemyStateChanged`
  (bind _asbp_enemy_aicontroller (cast `/Game/BootCamp/AI/BP_EnemyAIController` (`self.GetController`)))
  (if (`|EnumEquality` (`EnemyAIController.EnemyState` _asbp_enemy_aicontroller) "E_Patrol")
    (`self.SetPatrolSpeed`)
    (else
      (`self.SetFollowPlayerSpeed`))))

(event `self.Capsule.OnComponentBeginOverlap`
  (params (OverlappedComponent :type "PrimitiveComponent Object Reference") (OtherActor :type "Actor Object Reference") (OtherComp :type "PrimitiveComponent Object Reference") (OtherBodyIndex :type Integer) (bFromSweep :type Boolean) (SweepResult :type "HitResult Structure (by ref)"))
  (bind _ascapsule_collision (cast `CapsuleComponent` OtherComp))
  (cast `/Game/BootCamp/Blueprints/Character/BP_BootCampCharacter` (`ActorComponent.GetOwner` _ascapsule_collision))
  (bind _asbp_bcgame_instance (cast `/Game/BootCamp/Blueprints/BP_BCGameInstance` (`GameplayStatics.GetGameInstance`)))
  (set `/Game/BootCamp/Blueprints/BP_BCGameInstance.bDieByAGhost` true _asbp_bcgame_instance)
  (`KismetSystemLibrary.Delay` 0.2)
  (`GameplayStatics.OpenLevel` (`self.GameOver`)))

(fn `CheckCanDestroyEnemy`
  (if (< (`self.GetHealth`) 0.0)
    (`self.SetLifeSpan` 0.2)))

(fn `SetFollowPlayerSpeed`
  (set `CharacterMovementComponent.MaxWalkSpeed` (`self.FollowPlayerSpeed`) (`self.CharacterMovement`)))

(fn `SetPatrolSpeed`
  (set `CharacterMovementComponent.MaxWalkSpeed` (`self.PatrolWalkSpeed`) (`self.CharacterMovement`)))

(fn `SlowEnemySpeedAfterDamage`
  (set `CharacterMovementComponent.MaxWalkSpeed` (`self.DamageSpeed`) (`self.CharacterMovement`)))

(fn `UpdateHealthbar`
  (bind _asbp_enemy_health_bar (cast `/Game/BootCamp/Blueprints/UI/BP_EnemyHealthBar` (`WidgetComponent.GetUserWidgetObject` (`self.HealthBar`))))
  (`ProgressBar.SetPercent` (`/Game/BootCamp/Blueprints/UI/BP_EnemyHealthBar.EnemyHelathBar` _asbp_enemy_health_bar) (/ (`self.GetHealth`) (`self.MaxHealth`))))

(fn `UserConstructionScript`)