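; House actor for the BootCamp game with an openable door and a falling temperature that ends the game below zero.
; A box overlap by the player character shows a prompt and lets the input action flip-flop between open and close door timelines.
; A looping timer lowers temperature, and Tick loads the game-over map below zero.
; A second box toggles the campfire prompt and flag; IncreaseTemperature is not called here.
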(event `DecreaseTemperature`
  (set `self.CurrentTemperature` (- (`self.CurrentTemperature`) 2.0)))

(event `self.ReceiveBeginPlay`
  (`self.EnableInput` (`GameplayStatics.GetPlayerController` 0))
  (`KismetSystemLibrary.K2_SetTimerDelegate` (delegate `DecreaseTemperature`) 20.0 true 10.0))

(event `InputAction|OpenHouseDoor`
  (params (Key :type "Key Structure"))
  (:`Pressed`
    (if (`self.bCanOpenDoor`)
      (`self.OpenDoor`))))

(event `OpenDoor`
  (`/Engine/EditorBlueprintResources/StandardMacros.FlipFlop`
    (:`A`
      (bind (_direction _anglevalue) (`Timeline|OpenDoorTimeline` :!via `PlayFromStart`)
        (:`Update`
          (`SceneComponent.K2_SetRelativeRotation` (`self.SM_Door`) (`KismetMathLibrary.MakeRotator` 0.0 0.0 _anglevalue) false false))))
    (:`B`
      (bind (_direction_2 _anglevalue_2) (`Timeline|CloseDoor` :!via `PlayFromStart`)
        (:`Update`
          (`SceneComponent.K2_SetRelativeRotation` (`self.SM_Door`) (`KismetMathLibrary.MakeRotator` 0.0 0.0 _anglevalue_2) false false))))))

(event `self.Box.OnComponentBeginOverlap`
  (params (OverlappedComponent :type "PrimitiveComponent Object Reference") (OtherActor :type "Actor Object Reference") (OtherComp :type "PrimitiveComponent Object Reference") (OtherBodyIndex :type Integer) (bFromSweep :type Boolean) (SweepResult :type "HitResult Structure (by ref)"))
  (cast `/Game/BootCamp/Blueprints/Character/BP_BootCampCharacter` OtherActor)
  (`SceneComponent.SetHiddenInGame` (`self.OpenDoorActionText`) false false)
  (set `self.bCanOpenDoor` true))

(event `self.Box.OnComponentEndOverlap`
  (params (OverlappedComponent :type "PrimitiveComponent Object Reference") (OtherActor :type "Actor Object Reference") (OtherComp :type "PrimitiveComponent Object Reference") (OtherBodyIndex :type Integer))
  (cast `/Game/BootCamp/Blueprints/Character/BP_BootCampCharacter` OtherActor)
  (`SceneComponent.SetHiddenInGame` (`self.OpenDoorActionText`) true false)
  (set `self.bCanOpenDoor` false))

(event `IncreaseTemperature`
  (set `self.CurrentTemperature` (+ (`self.CurrentTemperature`) (`self.IncreaseTempValue`))))

(event `self.Box1.OnComponentBeginOverlap`
  (params (OverlappedComponent :type "PrimitiveComponent Object Reference") (OtherActor :type "Actor Object Reference") (OtherComp :type "PrimitiveComponent Object Reference") (OtherBodyIndex :type Integer) (bFromSweep :type Boolean) (SweepResult :type "HitResult Structure (by ref)"))
  (cast `/Game/BootCamp/Blueprints/Character/BP_BootCampCharacter` OtherActor)
  (`SceneComponent.SetHiddenInGame` (`self.CampFireActionText`) false false)
  (set `self.bCanUseCampfire` true))

(event `self.Box1.OnComponentEndOverlap`
  (params (OverlappedComponent :type "PrimitiveComponent Object Reference") (OtherActor :type "Actor Object Reference") (OtherComp :type "PrimitiveComponent Object Reference") (OtherBodyIndex :type Integer))
  (cast `/Game/BootCamp/Blueprints/Character/BP_BootCampCharacter` OtherActor)
  (`SceneComponent.SetHiddenInGame` (`self.CampFireActionText`) true false)
  (set `self.bCanUseCampfire` false))

(event `self.ReceiveTick`
  (params (DeltaSeconds :type "Float (single-precision)"))
  (if (< (`self.CurrentTemperature`) 0.0)
    (`GameplayStatics.OpenLevel` (`self.GameOverMap`))))

(fn `UserConstructionScript`)