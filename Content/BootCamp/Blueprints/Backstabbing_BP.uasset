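; Boot camp Blueprint that demonstrates a dot-product check for face-to-face versus backstabbing between a Player and an Object.
; BeginPlay places a text render above the Object and draws a debug line from it along world X.
; Tick prints the Player's forward dotted with normalized Player location minus Object forward vector (not Object location).
; Results beyond positive or negative thresholds set the label; values between leave it unchanged.
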(event `self.ReceiveBeginPlay`
  (bind _returnvalue (`self.K2_GetActorLocation` (`self.Object`)))
  (`SceneComponent.K2_SetWorldLocation` (`self.TextRender`) (+ (`self.K2_GetActorLocation` (`self.Object`)) (0.0 0.0 100.0)) false false)
  (`KismetSystemLibrary.DrawDebugLine` _returnvalue (+ _returnvalue (400.0 0.0 0.0)) (struct :`R` 0.69755 :`G` 0.100913 :`B` 0.527132 :`A` 1.0) 100.0))

(event `self.ReceiveTick`
  (params (DeltaSeconds :type "Float (single-precision)"))
  (bind _returnvalue (`KismetMathLibrary.Dot_VectorVector` (`self.GetActorForwardVector` (`self.Player`)) (`KismetMathLibrary.Normal` (- (`self.K2_GetActorLocation` (`self.Player`)) (`self.GetActorForwardVector` (`self.Object`))))))
  (`KismetSystemLibrary.PrintString` (`KismetStringLibrary.Conv_DoubleToString` _returnvalue) true true (struct :`G` 0.66 :`B` 1.0 :`A` 1.0) 0.5)
  ;[1 1 1] Quick check if the player is in front of the cube or behind
  (if (> _returnvalue 0.5)
    (set `self.TextVariable` "Face To Face")
    (`TextRenderComponent.K2_SetText` (`self.TextRender`) (`self.TextVariable`) :!label _label)
    (elif (< _returnvalue -0.5)
      (set `self.TextVariable` "Backstabbing")
      (goto _label))))

(fn `UserConstructionScript`)